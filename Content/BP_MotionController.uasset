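; VR motion controller for one hand, providing arc teleport, object grabbing and hand pose state.
; While the teleport button is held, Tick predicts a projectile arc and projects its hit onto the navmesh; release moves the owner there.
; Grab sphere-traces ahead and hands off to the hit actor's BP_GrabComponent.
; Construction sets the motion source from EHand, mirroring the left hand mesh via negative Z scale.
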(event `TeleportTrace`
  (bind _motioncontroller (`self.MotionController`))
  ;[1 1 1] 발사체의 궤적을 알수 있는 코드
  (bind (_outhit _outpathpositions _outlasttracedestination _returnvalue) (`GameplayStatics.Blueprint_PredictProjectilePath_ByTraceChannel` :`StartPos` (`SceneComponent.K2_GetComponentLocation` _motioncontroller) :`LaunchVelocity` (* (`SceneComponent.GetForwardVector` _motioncontroller) 650.0) :`ProjectileRadius` 3.0 :`TraceChannel` "ECC_WorldStatic" :`DrawDebugType` "ForOneFrame"))
  (bind (_projectedlocation _returnvalue_2) (`NavigationSystemV1.K2_ProjectPointToNavigation` (`NavigationSystemV1.GetNavigationSystem`) (`.Location` (`GameplayStatics.BreakHitResult` _outhit)) null null (0.0 0.0 0.0)))
  (bind _returnvalue_3 (and _returnvalue _returnvalue_2))
  (set `self.IsTeleport` _returnvalue_3)
  (if _returnvalue_3
    (`KismetSystemLibrary.DrawDebugSphere` _projectedlocation 100.0 12 (struct :`R` 1.0 :`B` 0.023477 :`A` 1.0))
    (set `self.Teleport Location` _projectedlocation)))

(event `self.ReceiveTick`
  (params (DeltaSeconds :type "Float (single-precision)"))
  (`/Engine/EditorBlueprintResources/StandardMacros.Gate` true :!label _label
    (:`Exit`
      (`self.TeleportTrace`))))

(event `TeleportButtom`
  (params (`Is Pressed` :type Boolean))
  (if `Is Pressed`
    (goto _label :!via `Open`)
    (else
      (`|ExecutionSequence`
        (:`then_0`
          (goto _label :!via `Close`))
        (:`then_1`
          (if (`self.IsTeleport`)
            (set `self.IsTeleport` false)
            (`self.K2_SetActorLocation` (`self.GetOwner`) (`self.Teleport Location`) false false)))))))

(event `Grab`
  (params (IsPressed :type Boolean))
  (bind _motioncontroller (`self.MotionController`))
  (bind _grabcomponent (`self.GrabComponent`))
  (bind _returnvalue (`SceneComponent.K2_GetComponentLocation` _motioncontroller))
  (if IsPressed
    (bind (_outhit _returnvalue_2) (`KismetSystemLibrary.SphereTraceSingleForObjects` :`Start` _returnvalue :`End` (+ _returnvalue (* (`SceneComponent.GetForwardVector` _motioncontroller) 50.0)) :`Radius` 20.0 :`ObjectTypes` (`|MakeArray` "ObjectTypeQuery2" "ObjectTypeQuery4" :!type "EObjectTypeQuery Enum") :`DrawDebugType` "ForDuration"))
    (if _returnvalue_2
      (bind _returnvalue_3 (`self.GetComponentByClass` (`.HitActor` (`GameplayStatics.BreakHitResult` _outhit)) "/Game/BP_GrabComponent.BP_GrabComponent_C"))
      (`/Engine/EditorBlueprintResources/StandardMacros.IsValid` _returnvalue_3
        (:`Is Valid`
          (bind _output_get (set `self.GrabComponent` _returnvalue_3))
          (`/Game/BP_GrabComponent.TryGrab` _output_get true (`self.QK_CustomHand`)))))
    (else
      (`/Engine/EditorBlueprintResources/StandardMacros.IsValid` _grabcomponent
        (:`Is Valid`
          (`/Game/BP_GrabComponent.TryGrab` _grabcomponent false (`self.QK_CustomHand`))
          (set `self.Hold` false))))))

(event `SetHandState`
  (params (HandState :type "/Game/Enum/E_HandPos Enum" :default "NewEnumerator0") (IsPressed :type Boolean))
  (switch `/Game/Enum/E_HandPos` HandState
    (:`NewEnumerator1`
      (set `self.Grip` IsPressed))
    (:`NewEnumerator2`
      (set `self.Pointing` IsPressed))
    (:`NewEnumerator3`
      (set `self.ThumbUp` IsPressed))
    (:`NewEnumerator4`
      (set `self.Hold` IsPressed))))

(event `self.ReceiveBeginPlay`
  (bind _asqk_custom_hand_skeleton_anim_blueprint (cast `/Game/Asset/Handle/Model/QK_CustomHand_Skeleton_AnimBlueprint` (`SkeletalMeshComponent.GetAnimInstance` (`self.QK_CustomHand`))))
  (set `self.HandAnim` _asqk_custom_hand_skeleton_anim_blueprint))

(fn `UserConstructionScript`
  (bind _ehand (`self.EHand`))
  (set `MotionControllerComponent.MotionSource` (`|GetEnumeratorName` _ehand) (`self.MotionController`))
  ;[1 1 1] 왼손 설정
  (if (`|EnumEquality` _ehand "Left")
    (`SceneComponent.SetRelativeScale3D` (`self.QK_CustomHand`) (1.05 1.05 -1.05))))